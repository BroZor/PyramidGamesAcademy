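; Collectible paper note (kartka) actor that the player picks up through its Interakcja (interaction) event.
; On interaction it destroys itself, plays a paper sound at its location and increments CollectiblesNumber on the BP_ThirdPersonCharacter.
; It then calls Otworz (open) on every Bp_drzwi_na_zebrane door in the level, without checking the count itself.
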(event EventBeginPlay)

(event Collision|EventActorBeginOverlap
  (params (OtherActor :type Actor%20Object%20Reference)))

(event EventTick
  (params (DeltaSeconds :type Float%20%28single-precision%29)))

(event EventInterakcja
  (Development|PrintString "usuwamy")
  (Actor|DestroyActor)
  (Audio|PlaySoundatLocation "/Game/moje/sound/paper.paper" (Transformation|GetActorLocation) "0, 0, 0" 1.0 1.0 0.0 0 0 0 0)
  (bind _returnvalue (Actor|GetActorOfClass "/Game/ThirdPerson/Blueprints/BP_ThirdPersonCharacter.BP_ThirdPersonCharacter_C"))
  (bind _result (Math|Integer|IncrementInt (Variables|/Game/ThirdPerson/Blueprints/BP_ThirdPersonCharacter.BP_ThirdPersonCharacter_C|GetCollectiblesNumber _returnvalue))
    (:%20%20
      (Variables|/Game/ThirdPerson/Blueprints/BP_ThirdPersonCharacter.BP_ThirdPersonCharacter_C|SetCollectiblesNumber _returnvalue _result)
      (bind _outactors (Actor|GetAllActorsOfClass "/Game/moje/Blueprints/bp_drzwi_na_zebrane.bp_drzwi_na_zebrane_C"))
      (for _array_element _outactors
        (Default|Otworz _array_element)))))

(fn ConstructionScript)