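; Door Blueprint that swings open or closed on Interakcja once the player has gathered enough collectibles.
; It compares CollectiblesNumber on the BP_ThirdPersonCharacter found in the level against its IloscKartek requirement.
; A Timeline plays or reverses based on IsOpen, lerping the StaticMesh yaw through a quarter turn and flipping IsOpen when finished.
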(event EventBeginPlay)

(event Collision|EventActorBeginOverlap
  (params (OtherActor :type Actor%20Object%20Reference)))

(event EventTick
  (params (DeltaSeconds :type Float%20%28single-precision%29)))

(event EventInterakcja
  (bind _returnvalue (Actor|GetActorOfClass "/Game/ThirdPerson/Blueprints/BP_ThirdPersonCharacter.BP_ThirdPersonCharacter_C"))
  (if (>= (Variables|/Game/ThirdPerson/Blueprints/BP_ThirdPersonCharacter.BP_ThirdPersonCharacter_C|GetCollectiblesNumber _returnvalue) (Variables|Default|GetiloscKartek))
    (if (Variables|Default|GetisOpen)
      (bind _drzwi_animacja (Timeline|Timeline Reverse)
        (:Update
          (Transformation|SetRelativeRotation (Variables|Default|GetStaticMesh) (Math|Rotator|MakeRotator 0.0 0.0 (Math|Float|Lerp 0.0 9e+01 _drzwi_animacja)) false false))
        (:Finished
          (Variables|Default|SetisOpen (not (Variables|Default|GetisOpen)))))
      (else
        (Timeline|Timeline Play)))))

(fn ConstructionScript)