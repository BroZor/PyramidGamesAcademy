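; Interactable door that opens only once the player character has collected at least the required number of notes (IloscKartek).
; The Interakcja event calls Otworz or Zamknij, which recheck that count and play or reverse the Drzwi timeline.
; The timeline swings the mesh yaw by 90 degrees, with an offset and optional mirroring, and flips IsOpen when finished.
; Opening enables overlaps on Box1 and the End_game_node trigger, while closing disables only Box1.
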(event EventBeginPlay)

(event Collision|EventActorBeginOverlap
  (params (OtherActor :type Actor%20Object%20Reference)))

(event EventTick
  (params (DeltaSeconds :type Float%20%28single-precision%29)))

(event EventInterakcja
  (if (Variables|Default|Getinteractable)
    (if (Variables|Default|GetisOpen)
      (CallFunction|Zamknij)
      (else
        (CallFunction|Otworz)))))

(fn ConstructionScript)

(fn Otworz
  (bind _returnvalue (Actor|GetActorOfClass "/Game/ThirdPerson/Blueprints/BP_ThirdPersonCharacter.BP_ThirdPersonCharacter_C"))
  (if (not (Variables|Default|GetisOpen))
    (if (>= (Variables|/Game/ThirdPerson/Blueprints/BP_ThirdPersonCharacter.BP_ThirdPersonCharacter_C|GetCollectiblesNumber _returnvalue) (Variables|Default|GetiloscKartek))
      (Audio|Components|Audio|Play (Variables|Default|Getdrzwi))
      (Variables|/Script/Engine.PrimitiveComponent|SetbGenerateOverlapEvents (Variables|Default|GetBox1) true)
      (bind _returnvalue_2 (Actor|GetActorOfClass "/Game/moje/end_game_node.end_game_node_C"))
      (Variables|/Script/Engine.PrimitiveComponent|SetbGenerateOverlapEvents (Variables|/Game/moje/end_game_node.end_game_node_C|GetBox _returnvalue_2) true))))

(fn Zamknij
  (bind _returnvalue (Actor|GetActorOfClass "/Game/ThirdPerson/Blueprints/BP_ThirdPersonCharacter.BP_ThirdPersonCharacter_C"))
  (if (Variables|Default|GetisOpen)
    (if (>= (Variables|/Game/ThirdPerson/Blueprints/BP_ThirdPersonCharacter.BP_ThirdPersonCharacter_C|GetCollectiblesNumber _returnvalue) (Variables|Default|GetiloscKartek))
      (Utilities|String|Reverse (Variables|Default|Getdrzwi))
      (Variables|/Script/Engine.PrimitiveComponent|SetbGenerateOverlapEvents (Variables|Default|GetBox1) false))))